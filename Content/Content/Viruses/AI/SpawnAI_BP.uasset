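; SpawnAI_BP is a placeable spawn point that creates one AI pawn from a configurable class when play begins.
; On BeginPlay it spawns the AIToSpawn class at the world location of its Sphere component.
; The construction script reads that class's default AI controller and writes the controller class name to a TextRender, labelling what each spawner produces.
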(event `self.ReceiveBeginPlay`
  (`AIBlueprintHelperLibrary.SpawnAIFromClass` (`self.AI_To_Spawn`) null (`SceneComponent.K2_GetComponentLocation` (`self.Sphere`))))

(fn `UserConstructionScript`
  (`TextRenderComponent.K2_SetText` (`self.TextRender`) (`KismetTextLibrary.Conv_StringToText` (`KismetSystemLibrary.GetClassDisplayName` (`.AIControllerClass` (defaults `/Game/Viruses/AI/SpawnAI_BP` (`self.AI_To_Spawn`)))))))